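; Base interactable actor that announces itself to the player character CH_MyChar in both first-person and top-down play.
; Overlap with the Interactable_Area component registers and unregisters it for FPS interaction messages.
; Cursor hover over the actor registers and unregisters it with the player character for top-down messages.
; SetHighlight toggles custom depth rendering on InteractableMesh for highlighting.
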(event OnComponentBeginOverlap(Interactable_Area)
  (params (OverlappedComponent :type Primitive%20Component%20Object%20Reference) (OtherActor :type Actor%20Object%20Reference) (OtherComp :type Primitive%20Component%20Object%20Reference) (OtherBodyIndex :type Integer) (bFromSweep :type Boolean) (SweepResult :type Hit%20Result%20Structure%20%28by%20ref%29))
  (bind _asch_my_char (Utilities|Casting|CastToCH_MyChar OtherActor))
  (Class|BPIInteract|RegisterInteractableFPS(Message) _asch_my_char self false))

(event OnComponentEndOverlap(Interactable_Area)
  (params (OverlappedComponent :type Primitive%20Component%20Object%20Reference) (OtherActor :type Actor%20Object%20Reference) (OtherComp :type Primitive%20Component%20Object%20Reference) (OtherBodyIndex :type Integer))
  (bind _asch_my_char (Utilities|Casting|CastToCH_MyChar OtherActor))
  (Class|BPIInteract|UnregisterInteractionFPS(Message) _asch_my_char self false))

(event MouseInput|EventActorEndCursorOver
  (bind _asch_my_char (Utilities|Casting|CastToCH_MyChar (Game|GetPlayerCharacter 0)))
  (Class|BPIInteract|UnregisterIteractableTD(Message) _asch_my_char self))

(event MouseInput|EventActorBeginCursorOver
  (bind _asch_my_char (Utilities|Casting|CastToCH_MyChar (Game|GetPlayerCharacter 0)))
  (Class|BPIInteract|RegisterInteractableTD(Message) _asch_my_char self))

(fn ConstructionScript)

(fn SetHighlight
  (params (highlight? :type Boolean))
  (Rendering|SetRenderCustomDepth (Variables|Default|GetInteractable_Mesh) highlight?))